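; Paper2D player character with a sprite body that moves on world axes from input and fires a weapon on the Fire action.
; Each tick it picks walk or idle animation from velocity and sets its direction from actor yaw.
; The construction script tilts the sprite to the spring arm's pitch and lowers it using a cosine of capsule half-height to compensate for the tilt.
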(event EventBeginPlay)

(event Collision|EventActorBeginOverlap
  (params (OtherActor :type Actor%20Object%20Reference)))

(event EventTick
  (params (DeltaSeconds :type Float%20%28single-precision%29))
  (|UpdateAnim))

(event Input|ActionEvents|InputActionFire
  (params (Key :type Key%20Structure :default "None"))
  (:Pressed
    (Class|MyPaperCharacter|FireWeapon)))

(event Input|AxisEvents|InputAxisXAxis
  (params (AxisValue :type Float%20%28single-precision%29))
  (Pawn|Input|AddMovementInput "0.000000,1.000000, 0" AxisValue false))

(event Input|AxisEvents|InputAxisYAxis
  (params (AxisValue :type Float%20%28single-precision%29))
  (Pawn|Input|AddMovementInput "-1.000000,0.000000, 0" AxisValue false))

(fn ConstructionScript
  (CallFunction|UpdateSpriteAngle))

(fn UpdateSpriteAngle
  (bind _sprite (Variables|Default|GetSprite))
  (bind _springarm (Variables|Default|GetSpringArm))
  (bind _capsulecomponent (Variables|Default|GetCapsuleComponent))
  (bind _returnvalue (Transformation|GetWorldRotation _springarm))
  (bind _capsulehalfheight (Variables|/Script/Engine.CapsuleComponent|GetCapsuleHalfHeight _capsulecomponent))
  (Transformation|SetWorldRotation _sprite (Math|Rotator|MakeRotator (.pitch _returnvalue) 0.0 -9e+01) false false)
  (Transformation|SetRelativeLocation _sprite (Math|Vector|MakeVector 0.0 0.0 (* (- _capsulehalfheight (* (Math|Trig|Cos(Degrees) (.pitch _returnvalue)) _capsulehalfheight)) -1.0)) false false))